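; Great spider enemy character with melee attacks, a floating health widget and a death sequence.
; ACStateAI holds health, armor, name and random level and receives damage; Tick refreshes the widget, turns it toward the player camera and checks for death.
; Attacks halt movement and play random montages, while events toggle left/right hitboxes, with DoOnce gates around random damage.
; Death plays an animation, disables capsule collision, hides the widget and destroys the actor after a delay.
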(event OnComponentBeginOverlap(L_Attack)
  (params (OverlappedComponent :type Primitive%20Component%20Object%20Reference) (OtherActor :type Actor%20Object%20Reference) (OtherComp :type Primitive%20Component%20Object%20Reference) (OtherBodyIndex :type Integer) (bFromSweep :type Boolean) (SweepResult :type Hit%20Result%20Structure%20%28by%20ref%29))
  ;[0.8854 0 0] урон
  (if (!= OtherActor self)
    (Utilities|FlowControl|DoOnce false
      (:Completed
        (Game|Damage|ApplyDamage OtherActor (Math|Random|RandomFloatinRange 5.0 2e+01) 0 0)))))

(event OnComponentBeginOverlap(R_Attack)
  (params (OverlappedComponent :type Primitive%20Component%20Object%20Reference) (OtherActor :type Actor%20Object%20Reference) (OtherComp :type Primitive%20Component%20Object%20Reference) (OtherBodyIndex :type Integer) (bFromSweep :type Boolean) (SweepResult :type Hit%20Result%20Structure%20%28by%20ref%29))
  ;[0.8854 0 0] урон
  (if (!= OtherActor self)
    (Utilities|FlowControl|DoOnce false
      (:Completed
        (Game|Damage|ApplyDamage OtherActor (Math|Random|RandomFloatinRange 5.0 2e+01) 0 0)))))

(event Custom|atack%20endet
  ;[1 1 1] атака
  (Utilities|Atack) ; enters at off
)

(event Custom|Attack
  ;[1 1 1] атака
  (Utilities|Atack))

(event Custom|cust%20desable%20collision%20R
  ;[0.8854 0 0] атака с права
  (Collision|SetCollisionEnabled (Variables|Default|GetR_Attack) "NoCollision"))

(event Custom|Refresh%20attack%20R
  ;[0.8854 0 0] урон
  (Utilities|FlowControl|DoOnce false) ; enters at Reset
)

(event Custom|cust%20enable%20collision%20R
  ;[0.8854 0 0] атака с права
  (Collision|SetCollisionEnabled (Variables|Default|GetR_Attack) "QueryOnly")
  (CallFunction|RefreshAttackL))

(event Custom|cust%20enable%20collision%20L
  ;[0.8854 0 0] атака слева
  (Collision|SetCollisionEnabled (Variables|Default|GetL_Attack) "QueryOnly")
  (CallFunction|RefreshAttackR))

(event Custom|cust%20desable%20collision%20L
  ;[0.8854 0 0] атака слева
  (Collision|SetCollisionEnabled (Variables|Default|GetL_Attack) "NoCollision"))

(event Custom|Refresh%20attack%20l
  ;[0.8854 0 0] урон
  (Utilities|FlowControl|DoOnce false) ; enters at Reset
)

(event EventBeginPlay
  (Default|SETHPAI (Variables|Default|GetAC_State_AI) 3e+02 3e+02)
  (Default|SETARMORAI (Variables|Default|GetAC_State_AI) 1.0 1.0)
  (Default|SETNAMELEVEL (Variables|Default|GetAC_State_AI) "SPIDER" (Math|Random|RandomInteger 5))
  (CallFunction|UIHP)
  (CallFunction|MaxSpeed))

(event Game|Damage|EventAnyDamage
  (params (Damage :type Float%20%28single-precision%29) (DamageType :type Damage%20Type%20Object%20Reference) (InstigatedBy :type Controller%20Object%20Reference) (DamageCauser :type Actor%20Object%20Reference))
  (if (not (Variables|Default|Getis%20dead%20?))
    (Variables|Default|SetDamage Damage)
    (Default|INDAMAGEAI (Variables|Default|GetAC_State_AI) (Variables|Default|GetDamage))
    (Development|PrintString "/////////////////////" true true "(R=1.000000,G=1.000000,B=0.000000,A=1.000000)")))

(event EventTick
  (params (DeltaSeconds :type Float%20%28single-precision%29))
  (CallFunction|ROTATEWIDGETSAI)
  (CallFunction|HPARMOR)
  (Utilities|IsDead))

(fn ConstructionScript)

(fn UIHP
  ;[1 1 1] виджет НР
  (Variables|Default|SetHealth%20ai (.AsW%20Health%20AI (Utilities|Casting|CastToW_Health_AI (UserInterface|GetUserWidgetObject (Variables|Default|GetUI_HP))))))

(fn HPARMOR
  (bind (_name _levl _hp_max _hp_current _hp_progres_bar) (Default|GETHPARMORAI (Variables|Default|GetAC_State_AI)))
  (Rendering|Components|TextRender|SetText (Variables|/Game/Widgets/Game/widgets_styte_AI/W_Health_AI.W_Health_AI_C|Getname_text (Variables|Default|GetHealth%20ai)) _name)
  (Rendering|Components|TextRender|SetText (Variables|/Game/Widgets/Game/widgets_styte_AI/W_Health_AI.W_Health_AI_C|Getlevel_text (Variables|Default|GetHealth%20ai)) (Utilities|Text|FormatText "Level [ {level} ]" _levl))
  (Rendering|Components|TextRender|SetText (Variables|/Game/Widgets/Game/widgets_styte_AI/W_Health_AI.W_Health_AI_C|Gethp_text (Variables|Default|GetHealth%20ai)) (Utilities|Text|FormatText "{max} / {Current}" _hp_max _hp_current))
  (Progress|SetPercent (Variables|/Game/Widgets/Game/widgets_styte_AI/W_Health_AI.W_Health_AI_C|GetHP_Bare (Variables|Default|GetHealth%20ai)) _hp_progres_bar))

(fn ROTATEWIDGETSAI
  (Transformation|SetWorldRotation (Variables|Default|GetUI_HP) (Math|Rotator|FindLookatRotation (Transformation|GetWorldLocation (Variables|Default|GetUI_HP)) (Transformation|GetWorldLocation (Variables|/Game/charecter/Player/ThirdPersonCharacter.ThirdPersonCharacter_C|GetFollowCamera (.AsThird%20Person%20Character (Utilities|Casting|CastToThirdPersonCharacter (Game|GetPlayerCharacter 0)))))) false false))

(fn MaxSpeed
  ;[1 1 1] начальная скорость
  (Variables|Default|Setmax%20start%20speed (Variables|/Script/Engine.CharacterMovementComponent|GetMaxWalkSpeed (Variables|Character|GetCharacterMovement))))

(fn MaxWalkSpeed
  (params (Condition :type Boolean))
  (if Condition
    (Variables|/Script/Engine.CharacterMovementComponent|SetMaxWalkSpeed (Variables|Character|GetCharacterMovement) 0.0)
    (else
      (Variables|/Script/Engine.CharacterMovementComponent|SetMaxWalkSpeed (Variables|Character|GetCharacterMovement) (Variables|Default|Getmax%20start%20speed)))))

(fn BotDead!?
  (if (Variables|/Game/charecter/ai/AC_State_AI.AC_State_AI_C|GetIs%20Death%20AI? (Variables|Default|GetAC_State_AI))
    (Default|CustBPDeathAnim (.AsSK%20Greater%20Spider%20Anim (Utilities|Casting|CastToSK_Greater_Spider_Anim (Components|SkeletalMesh|GetAnimInstance (Variables|Character|GetMesh)))))
    (Animation|StopAnimMontage "/Game/InfinityBladeAdversaries/Enemy/Enemy_Great_Spider/Enemy_SpiderGreater_Animation/Attack_Melee_B_Montage.Attack_Melee_B_Montage")
    (Animation|StopAnimMontage "/Game/InfinityBladeAdversaries/Enemy/Enemy_Great_Spider/Enemy_SpiderGreater_Animation/Attack_Melee_C_Montage.Attack_Melee_C_Montage")
    (Animation|StopAnimMontage "/Game/InfinityBladeAdversaries/Enemy/Enemy_Great_Spider/Enemy_SpiderGreater_Animation/Attack_Melee_Montage.Attack_Melee_Montage")
    (Collision|SetCollisionEnabled (Variables|Collision|GetCapsuleComponent) "NoCollision")
    (return)))