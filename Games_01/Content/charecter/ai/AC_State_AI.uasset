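; Actor component that holds an AI character's state: name, level, health, armor and death flag.
; Setters initialize the values, clamping level to at least 1, and a getter returns UI-ready text and normalized bar values.
; Damage drains armor first; when armor is zero after a hit, that hit's full damage also reduces HP.
; Tick triggers death when HP reaches zero, blocking further damage; Respawn is an empty stub.
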(event Custom|Respawn)

(event Custom|Cust_Is_dead
  (Variables|SYSTEM|DAMAGE|SetIs%20Death%20AI? true))

(event EventTick
  (params (DeltaSeconds :type Float%20%28single-precision%29))
  (if (and (<= (Variables|SYSTEM|HP|GetHP%20Current%20AI) 0.0) (not (Variables|SYSTEM|DAMAGE|GetIs%20Death%20AI?)))
    (CallFunction|CustIsDead)))

(fn GETHPARMORAI
  (return (Variables|SYSTEM|NAMELEVEL|GetNAME) (Utilities|Text|ToText(Integer) (Variables|SYSTEM|NAMELEVEL|GetLEVEL)) (Utilities|Text|ToText(Integer) (Math|Float|Truncate (Variables|SYSTEM|HP|GetHP%20Max%20AI))) (Utilities|Text|ToText(Integer) (Math|Float|Truncate (Variables|SYSTEM|HP|GetHP%20Current%20AI))) (Math|Float|NormalizetoRange (Variables|SYSTEM|HP|GetHP%20Current%20AI) 0.0 (Variables|SYSTEM|HP|GetHP%20Max%20AI)) (Utilities|Text|ToText(Integer) (Math|Float|Truncate (Variables|SYSTEM|ARMOR|Getarmor%20Max%20AI))) (Utilities|Text|ToText(Integer) (Math|Float|Truncate (Variables|SYSTEM|ARMOR|Getarmor%20Current%20AI))) (Math|Float|NormalizetoRange (Variables|SYSTEM|ARMOR|Getarmor%20Current%20AI) 0.0 (Variables|SYSTEM|ARMOR|Getarmor%20Max%20AI))))

(fn SETARMORAI
  (params (ARMOR%20MAX :type Float%20%28single-precision%29) (ARMOR%20Current :type Float%20%28single-precision%29))
  (Variables|SYSTEM|ARMOR|Setarmor%20Max%20AI ARMOR%20MAX)
  (Variables|SYSTEM|ARMOR|Setarmor%20Current%20AI ARMOR%20Current)
  (return (Variables|SYSTEM|ARMOR|Getarmor%20Max%20AI) (Variables|SYSTEM|ARMOR|Getarmor%20Current%20AI)))

(fn SETHPAI
  (params (HP%20MAX :type Float%20%28single-precision%29) (HP%20CURENT :type Float%20%28single-precision%29))
  (Variables|SYSTEM|HP|SetHP%20Max%20AI HP%20MAX)
  (Variables|SYSTEM|HP|SetHP%20Current%20AI HP%20CURENT)
  (return (Variables|SYSTEM|HP|GetHP%20Max%20AI) (Variables|SYSTEM|HP|GetHP%20Current%20AI)))

(fn INDAMAGEAI
  (params (damage :type Float%20%28single-precision%29))
  (LocalVariables|SetL%20damage damage)
  (if (not (Variables|SYSTEM|DAMAGE|GetIs%20Death%20AI?))
    (Variables|SYSTEM|ARMOR|Setarmor%20Current%20AI (Math|Float|SelectFloat 0.0 (- (Variables|SYSTEM|ARMOR|Getarmor%20Current%20AI) (LocalVariables|GetL%20damage)) (>= (LocalVariables|GetL%20damage) (Variables|SYSTEM|ARMOR|Getarmor%20Current%20AI))))
    (if (== (Variables|SYSTEM|ARMOR|Getarmor%20Current%20AI) 0.0)
      (Variables|SYSTEM|HP|SetHP%20Current%20AI (Math|Float|SelectFloat 0.0 (- (Variables|SYSTEM|HP|GetHP%20Current%20AI) (LocalVariables|GetL%20damage)) (>= (LocalVariables|GetL%20damage) (Variables|SYSTEM|HP|GetHP%20Current%20AI)))))))

(fn SETNAMELEVEL
  (params (NAME :type Text) (LEVEL :type Integer))
  (Variables|SYSTEM|NAMELEVEL|SetNAME NAME)
  (if (<= LEVEL 0)
    (Variables|SYSTEM|NAMELEVEL|SetLEVEL 1)
    (else
      (Variables|SYSTEM|NAMELEVEL|SetLEVEL LEVEL)))
  (return (Variables|SYSTEM|NAMELEVEL|GetNAME) (Variables|SYSTEM|NAMELEVEL|GetLEVEL)))